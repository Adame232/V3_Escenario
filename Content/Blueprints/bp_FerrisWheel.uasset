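; Ferris wheel actor that starts turning on BeginPlay and keeps its baskets level as the wheel rotates.
; A start timeline ramps the rotation timeline's play rate from zero up to RotationRate, easing the wheel into motion.
; The rotation timeline lerps the wheel's relative rotation through 360 degrees.
; Each update also resets the baskets' world rotation to the actor's roll and yaw, leaving pitch at zero.
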(event `self.ReceiveBeginPlay`
  (`self.EventStartWheel`)
  (`self.EventRotateWheel`))

(event `EventStartWheel`
  ;[1 0.9192 0.225] Start Rotation
  (bind (_direction _alpha) (`Timeline|TM_Wheel_Start` :!via `PlayFromStart`)
    (:`Update`
      (set `self.CurrentRate` (`KismetMathLibrary.Lerp` 0.0 (`self.RotationRate`) _alpha))
      (`TimelineComponent.SetPlayRate` (`self.TM_Wheel_Rotate`) (`self.CurrentRate`)))))

(event `EventRotateWheel`
  ;[1 0.9192 0.225] Rotation
  (`TimelineComponent.SetPlayRate` (`self.TM_Wheel_Rotate`) (`self.CurrentRate`))
  (bind (_direction _alpha) (`Timeline|TM_Wheel_Rotate`)
    (:`Update`
      (`SceneComponent.K2_SetRelativeRotation` (`self.Wheel_01`) (`KismetMathLibrary.RLerp` (struct) (struct :`Pitch` 360.0) _alpha) false false)
      (`self.ROTATE BASKETS`))))

(event `ROTATE BASKETS`
  (bind (_returnvalue_roll _returnvalue_pitch _returnvalue_yaw) (`KismetMathLibrary.BreakRotator` (`self.K2_GetActorRotation`)))
  (`SceneComponent.K2_SetWorldRotation` (`self.BasketCase_1`) (`KismetMathLibrary.MakeRotator` _returnvalue_roll 0.0 _returnvalue_yaw) false false)
  (`SceneComponent.K2_SetWorldRotation` (`self.BasketCase_2`) (`KismetMathLibrary.MakeRotator` _returnvalue_roll 0.0 _returnvalue_yaw) false false)
  (`SceneComponent.K2_SetWorldRotation` (`self.BasketCase_3`) (`KismetMathLibrary.MakeRotator` _returnvalue_roll 0.0 _returnvalue_yaw) false false)
  (`SceneComponent.K2_SetWorldRotation` (`self.BasketCase_4`) (`KismetMathLibrary.MakeRotator` _returnvalue_roll 0.0 _returnvalue_yaw) false false)
  (`SceneComponent.K2_SetWorldRotation` (`self.BasketCase_6`) (`KismetMathLibrary.MakeRotator` _returnvalue_roll 0.0 _returnvalue_yaw) false false)
  (`SceneComponent.K2_SetWorldRotation` (`self.BasketCase_7`) (`KismetMathLibrary.MakeRotator` _returnvalue_roll 0.0 _returnvalue_yaw) false false)
  (`SceneComponent.K2_SetWorldRotation` (`self.BasketCase_9`) (`KismetMathLibrary.MakeRotator` _returnvalue_roll 0.0 _returnvalue_yaw) false false)
  (`SceneComponent.K2_SetWorldRotation` (`self.BasketCase_10`) (`KismetMathLibrary.MakeRotator` _returnvalue_roll 0.0 _returnvalue_yaw) false false)
  (`SceneComponent.K2_SetWorldRotation` (`self.BasketCase_11`) (`KismetMathLibrary.MakeRotator` _returnvalue_roll 0.0 _returnvalue_yaw) false false)
  (`SceneComponent.K2_SetWorldRotation` (`self.BasketCase_12`) (`KismetMathLibrary.MakeRotator` _returnvalue_roll 0.0 _returnvalue_yaw) false false))

(fn `UserConstructionScript`)