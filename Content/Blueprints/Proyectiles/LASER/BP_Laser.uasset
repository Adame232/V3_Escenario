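; BP_Laser is a laser hazard that damages the first-person character when it enters the capsule trigger.
; Any overlap activates the particle system and plays the laser sound at the sphere's location; ending the overlap deactivates the particles.
; For a FirstPersonCharacter, a short delay precedes a single fixed deduction from Salud (health), even if it has left the capsule.
; The character's RespawnActor is called when health reaches zero or below.
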(event `self.Capsule.OnComponentBeginOverlap`
  (params (OverlappedComponent :type "PrimitiveComponent Object Reference") (OtherActor :type "Actor Object Reference") (OtherComp :type "PrimitiveComponent Object Reference") (OtherBodyIndex :type Integer) (bFromSweep :type Boolean) (SweepResult :type "HitResult Structure (by ref)"))
  (`ActorComponent.Activate` (`self.ParticleSystem`) false)
  (`GameplayStatics.PlaySoundAtLocation` "/Game/Blueprints/Proyectiles/LASER/Laser_Cue.Laser_Cue" (`SceneComponent.K2_GetComponentLocation` (`self.Sphere`)) (struct) 1.0 1.0 0.0 null null null)
  (bind _asfirst_person_character (cast `/Game/FirstPersonBP/Blueprints/FirstPersonCharacter` OtherActor))
  (`KismetSystemLibrary.Delay` 0.25)
  (bind _output_get (set `/Game/FirstPersonBP/Blueprints/FirstPersonCharacter.Salud` (- (`/Game/FirstPersonBP/Blueprints/FirstPersonCharacter.Salud` _asfirst_person_character) 15.0) _asfirst_person_character))
  (if (<= _output_get 0.0)
    (`/Game/FirstPersonBP/Blueprints/FirstPersonCharacter.RespawnActor` _asfirst_person_character)))

(event `self.Capsule.OnComponentEndOverlap`
  (params (OverlappedComponent :type "PrimitiveComponent Object Reference") (OtherActor :type "Actor Object Reference") (OtherComp :type "PrimitiveComponent Object Reference") (OtherBodyIndex :type Integer))
  (`ActorComponent.Deactivate` (`self.ParticleSystem`)))

(fn `UserConstructionScript`)