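; A test damage actor that hurts the first-person character when it enters the actor's Box trigger.
; On overlap, it subtracts a fixed amount from the character's shield (Escudo) if any remains, otherwise from health (Salud), clamping each at zero.
; Damage beyond the remaining shield does not carry over to health, and each overlap applies a single hit with no tick or timer.
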(event `self.Box.OnComponentBeginOverlap`
  (params (OverlappedComponent :type "PrimitiveComponent Object Reference") (OtherActor :type "Actor Object Reference") (OtherComp :type "PrimitiveComponent Object Reference") (OtherBodyIndex :type Integer) (bFromSweep :type Boolean) (SweepResult :type "HitResult Structure (by ref)"))
  (bind _asfirst_person_character (cast `/Game/FirstPersonBP/Blueprints/FirstPersonCharacter` OtherActor))
  (bind _escudo (`/Game/FirstPersonBP/Blueprints/FirstPersonCharacter.Escudo` _asfirst_person_character))
  (if (> _escudo 0.0)
    (set `/Game/FirstPersonBP/Blueprints/FirstPersonCharacter.Escudo` (- _escudo 10.0) _asfirst_person_character)
    (if (< _escudo 0.0)
      (set `/Game/FirstPersonBP/Blueprints/FirstPersonCharacter.Escudo` 0.0 _asfirst_person_character))
    (else
      (bind _salud (`/Game/FirstPersonBP/Blueprints/FirstPersonCharacter.Salud` _asfirst_person_character))
      (set `/Game/FirstPersonBP/Blueprints/FirstPersonCharacter.Salud` (- _salud 10.0) _asfirst_person_character)
      (if (< _salud 0.0)
        (set `/Game/FirstPersonBP/Blueprints/FirstPersonCharacter.Salud` 0.0 _asfirst_person_character)))))

(fn `UserConstructionScript`)