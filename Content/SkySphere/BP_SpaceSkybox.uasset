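; BP_SpaceSkybox is a space skybox actor that applies a configurable material to its SkySphere component.
; It passes its Power, StarBrightness and SceneBrightness variables to scalar parameters of the same names to tune the sky's look.
; The construction script and BeginPlay run identical setup, so the settings apply both on construction and when play starts.
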(event `self.ReceiveBeginPlay`
  (`PrimitiveComponent.SetMaterial` (`self.SkySphere`) 0 (`self.Material`))
  (`KismetMaterialLibrary.SetScalarParameterValue` null "Power" (`self.Power`))
  (`KismetMaterialLibrary.SetScalarParameterValue` null "StarBrightness" (`self.StarBrightness`))
  (`KismetMaterialLibrary.SetScalarParameterValue` null "SceneBrightness" (`self.SceneBrightness`)))

(fn `UserConstructionScript`
  (`PrimitiveComponent.SetMaterial` (`self.SkySphere`) 0 (`self.Material`))
  (`KismetMaterialLibrary.SetScalarParameterValue` null "Power" (`self.Power`))
  (`KismetMaterialLibrary.SetScalarParameterValue` null "StarBrightness" (`self.StarBrightness`))
  (`KismetMaterialLibrary.SetScalarParameterValue` null "SceneBrightness" (`self.SceneBrightness`)))