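; BP_SpaceSkybox is a space skybox actor that applies a chosen material to its SkySphere component.
; It writes its Power, StarBrightness and SceneBrightness variables as scalars into the PC_SpaceSkybox Material Parameter Collection.
; The Construction Script and BeginPlay run identical logic, so the look updates in the editor and is reapplied when play starts.
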(event `self.ReceiveBeginPlay`
  (`PrimitiveComponent.SetMaterial` (`self.SkySphere`) 0 (`self.Material`))
  (`KismetMaterialLibrary.SetScalarParameterValue` "/Game/SkySphere/Texture/PC_SpaceSkybox.PC_SpaceSkybox" "Power" (`self.Power`))
  (`KismetMaterialLibrary.SetScalarParameterValue` "/Game/SkySphere/Texture/PC_SpaceSkybox.PC_SpaceSkybox" "StarBrightness" (`self.StarBrightness`))
  (`KismetMaterialLibrary.SetScalarParameterValue` "/Game/SkySphere/Texture/PC_SpaceSkybox.PC_SpaceSkybox" "SceneBrightness" (`self.SceneBrightness`)))

(fn `UserConstructionScript`
  (`PrimitiveComponent.SetMaterial` (`self.SkySphere`) 0 (`self.Material`))
  (`KismetMaterialLibrary.SetScalarParameterValue` "/Game/SkySphere/Texture/PC_SpaceSkybox.PC_SpaceSkybox" "Power" (`self.Power`))
  (`KismetMaterialLibrary.SetScalarParameterValue` "/Game/SkySphere/Texture/PC_SpaceSkybox.PC_SpaceSkybox" "StarBrightness" (`self.StarBrightness`))
  (`KismetMaterialLibrary.SetScalarParameterValue` "/Game/SkySphere/Texture/PC_SpaceSkybox.PC_SpaceSkybox" "SceneBrightness" (`self.SceneBrightness`)))