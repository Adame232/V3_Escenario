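; BP_Spawner is an actor that spawns a grid of BP_Cube actors at its root location when play begins.
; A 2D grid macro sized by Rows and Columns spawns one cube at each cell center.
; An alternate recursive Redraw event chains cubes through each one's LeftLocation and FrontLocation instead, but BeginPlay does not call it.
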(event `Redraw`
  ;[1 1 1] Alternate Event
  (for _ (range (+ (`self.Rows`) 1))
    (bind _returnvalue (`|SpawnActorFromClass` "/Game/Platform/Materials/BP_Cube.BP_Cube_C" (`KismetMathLibrary.MakeTransform` (`self.NextCube`) (struct) (`self.ScaleCube`)) "Undefined" "OverrideRootScale" null null))
    (set `self.NextCube` (`/Game/Platform/Materials/BP_Cube.Left_Location` _returnvalue))
    (`/Engine/EditorBlueprintResources/StandardMacros.DoOnce` false
      (:`Completed`
        (set `self.FrontCube` (`/Game/Platform/Materials/BP_Cube.Front_Location` _returnvalue)))))
  (bind _returnvalue_2 (`|SpawnActorFromClass` "/Game/Platform/Materials/BP_Cube.BP_Cube_C" (`KismetMathLibrary.MakeTransform` (`self.FrontCube`) (struct) (`self.ScaleCube`)) "Undefined" "OverrideRootScale" null null))
  (set `self.NextCube` (`/Game/Platform/Materials/BP_Cube.Left_Location` _returnvalue_2))
  (set `self.FrontCube` (`/Game/Platform/Materials/BP_Cube.Front_Location` _returnvalue_2))
  (if (<= (`self.CountHelper`) (`self.Columns`))
    (set `self.CountHelper` (+ (`self.CountHelper`) 1))
    (`self.Redraw`)))

(event `self.ReceiveBeginPlay`
  (bind _output_get (set `self.NextCube` (`SceneComponent.K2_GetComponentLocation` (`self.DefaultSceneRoot`))))
  (bind (_current_point _total_points _0_1_phase _poly_center) (`/Engine/ArtTools/RenderToTexture/Macros/RenderToTextureMacros.2D Grid Execution Macro` 100.0 _output_get (`self.Rows`) (`self.Columns`))
    (:`Per Poly Execution`
      (`|SpawnActorFromClass` "/Game/Platform/Materials/BP_Cube.BP_Cube_C" (`KismetMathLibrary.MakeTransform` _poly_center) "Undefined" "OverrideRootScale" null null))))

(fn `UserConstructionScript`)